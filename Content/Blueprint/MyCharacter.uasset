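; MyCharacter is a player Character Blueprint that handles movement input and weapon firing.
; Forward, backward, left and right axis events feed AddMovementInput along the player camera manager's forward and right vectors, making movement camera-relative.
; Releasing the left mouse button calls FireWeapon, whose logic is not defined in this graph.
; BeginPlay, Tick, overlap and the construction script are empty.
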(event `InputAxis|MoveForward`
  (params (AxisValue :type "Float (single-precision)"))
  (`self.AddMovementInput` (`self.GetActorForwardVector` (`GameplayStatics.GetPlayerCameraManager` 0)) AxisValue))

(event `Key|LeftMouseButton`
  (params (Key :type "Key Structure"))
  (:`Released`
    (`self.FireWeapon`)))

(event `InputAxis|MoveBackward`
  (params (AxisValue :type "Float (single-precision)"))
  (`self.AddMovementInput` (`self.GetActorForwardVector` (`GameplayStatics.GetPlayerCameraManager` 0)) AxisValue))

(event `InputAxis|MoveRight`
  (params (AxisValue :type "Float (single-precision)"))
  (`self.AddMovementInput` (`self.GetActorRightVector` (`GameplayStatics.GetPlayerCameraManager` 0)) AxisValue))

(event `InputAxis|MoveLeft`
  (params (AxisValue :type "Float (single-precision)"))
  (`self.AddMovementInput` (`self.GetActorRightVector` (`GameplayStatics.GetPlayerCameraManager` 0)) AxisValue))

(fn `UserConstructionScript`)